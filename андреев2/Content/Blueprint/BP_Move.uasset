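; Moves a Valdai component along a spline and carries the VR pawn with it as a scripted ride.
; Tick stays off until the VRPawn overlaps LeverStart, then advances a distance by Splinespeed each frame.
; The component takes the spline's local X, Y and offset yaw.
; The pawn is teleported using a hard-coded axis swap, scale and offset of that local point instead of being attached.
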(event `self.ReceiveBeginPlay`
  (`self.SetActorTickEnabled` false))

(event `self.ReceiveTick`
  (params (DeltaSeconds :type "Float (single-precision)"))
  (bind _distance (`self.distance`))
  (bind _returnvalue (`SplineComponent.GetTransformAtDistanceAlongSpline` (`self.Spline`) _distance "Local" false))
  (set `self.distance` (+ (* DeltaSeconds (`self.splinespeed`)) _distance))
  (`SceneComponent.K2_SetRelativeTransform` (`self.ультракрутойвалдай42`) (`KismetMathLibrary.MakeTransform` (`KismetMathLibrary.MakeVector` (.x (.location _returnvalue)) (.y (.location _returnvalue))) (`KismetMathLibrary.MakeRotator` 0.0 0.0 (+ (.yaw (.rotation _returnvalue)) -90.0))) false true)
  (bind _returnvalue_2 (`GameplayStatics.GetActorOfClass` "/Game/VRTemplate/Blueprints/VRPawn.VRPawn_C"))
  (`self.K2_SetActorLocation` _returnvalue_2 (`KismetMathLibrary.MakeVector` (+ (* (.y (.location _returnvalue)) 2.0) -29000.0) (+ (* (.x (.location _returnvalue)) -2.0) -65000.0) (+ (.z (.location _returnvalue)) 720.0)) false true))

(event `self.LeverStart.OnComponentBeginOverlap`
  (params (OverlappedComponent :type "PrimitiveComponent Object Reference") (OtherActor :type "Actor Object Reference") (OtherComp :type "PrimitiveComponent Object Reference") (OtherBodyIndex :type Integer) (bFromSweep :type Boolean) (SweepResult :type "HitResult Structure (by ref)"))
  (if (`GameplayStatics.ObjectIsA` OtherActor "/Game/VRTemplate/Blueprints/VRPawn.VRPawn_C")
    (`self.SetActorTickEnabled` true)))

(fn `UserConstructionScript`)